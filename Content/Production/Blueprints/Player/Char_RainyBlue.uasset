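; RainyBlue player character with single-axis movement, jump and interaction, driven by the RB gameplay state.
; During gameplay idle, Tick updates left/right facing from X velocity and picks the closest actor in front with an interactable component via sphere overlap and dot product.
; If interactable, that component is notified and cached for the interact input.
; A timeline blends spring arm and FOV, reversing to close-up for cinematics, dialogue and minigames.
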(event `self.ReceiveTick`
  (params (DeltaSeconds :type "Float (single-precision)"))
  (switch `EGameplayState` (`/Game/Production/Blueprints/GameMode/BPF_GameplayUtil.GetRBGameplayState`)
    (:`EV_InGameplayIdle`
      (`self.UpdateFacingDir`)
      (bind (_actor _interactablecomponent) (`self.CheckBestInteractableObject` (`self.InteractionCheckRange`)))
      (set `self.BestInteractableComponent` _interactablecomponent))))

(event `/Game/Production/Blueprints/GameMode/BPI_Movement.OnMoveRight`
  (params (AxisVal :type "Float (single-precision)"))
  (`self.AddMovementInput` (`self.GetActorForwardVector`) AxisVal))

(event `/Game/Production/Blueprints/GameMode/BPI_Movement.OnJump`
  (`self.Jump`))

(event `/Game/Production/Blueprints/GameMode/BPI_Interaction.OnInteract`
  (params (Instigator :type "Actor Object Reference"))
  (message `/Game/Production/Blueprints/GameMode/BPI_Interaction.OnInteract` (`self.BestInteractableComponent`) self))

(event `/Game/Production/Blueprints/GameMode/BPI_GameplayState.InitializeOnGameplayState`
  (params (NewState :type "EGameplayState Enum" :default "EV_InGameplayIdle"))
  (switch `EGameplayState` NewState
    (:`EV_InGameplayIdle`
      (bind (_direction _timeline) (`Timeline|CameraInitializationTimeline` :!label _label)
        (:`Update`
          (`self.CameraInitializationTick` _timeline))))
    (:`EV_InCinematic`
      (goto _label :!via `Reverse`))
    (:`EV_InDialogue`
      (goto _label :!via `Reverse`))
    (:`EV_InMiniGame`
      (goto _label :!via `Reverse`))))

(fn `CameraInitializationTick`
  (params (Alpha :type "Float (double-precision)"))
  (set `SpringArmComponent.TargetArmLength` (`KismetMathLibrary.Lerp` (`self.CloseCamSpringArm`) (`self.InitialCamSpringArm`) Alpha) (`self.SpringArm`))
  (`CameraComponent.SetFieldOfView` (`self.Camera`) (`KismetMathLibrary.Lerp` (`self.CloseCamFOV`) (`self.InitialCamFOV`) Alpha)))

(fn `CheckBestInteractableObject`
  (params (Range :type "Float (double-precision)" :default 128.0))
  (returns (Actor :type "Actor Object Reference") (InteractableComponent :type "/Game/Production/Blueprints/Components/BPAC_InteractableComponent Object Reference"))
  (locals (InteractableObjectsInRange :type "Array of Actor Object Reference") (ClosestActor :type "Actor Object Reference") (ClosestDist :type "Float (double-precision)"))
  (bind _closestactor (`local.ClosestActor`))
  (bind _returnvalue (`self.GetComponentByClass` _closestactor "/Game/Production/Blueprints/Components/BPAC_InteractableComponent.BPAC_InteractableComponent_C"))
  ;[1 1 1] Get Everything In Range
  (bind (_outactors _returnvalue_2) (`KismetSystemLibrary.SphereOverlapActors` (`self.K2_GetActorLocation`) Range (`|MakeArray` "ObjectTypeQuery1" "ObjectTypeQuery2" "ObjectTypeQuery4" :!type "EObjectTypeQuery Enum") null (`|MakeArray` self :!type "Actor Object Reference")))
  (if _returnvalue_2
    ;[1 1 1] Check has component implementing BPI Interactable interface -> BPAC_InteractableComponent
    (for _array_element _outactors
      (if (> (`KismetArrayLibrary.Array_Length` (`self.K2_GetComponentsByClass` _array_element "/Game/Production/Blueprints/Components/BPAC_InteractableComponent.BPAC_InteractableComponent_C")) 0)
        (if (>= (`KismetMathLibrary.Dot_VectorVector` (- (`self.K2_GetActorLocation` _array_element) (`self.K2_GetActorLocation`)) (`SceneComponent.GetForwardVector` (`self.FacingDir`))) 0.0)
          (`KismetArrayLibrary.Array_AddUnique` (`local.InteractableObjectsInRange`) _array_element))))
    (set `local.ClosestDist` Range)
    ;[1 1 1] Second Pass to filter out most close target
    (for _array_element_2 (`local.InteractableObjectsInRange`)
      (bind _returnvalue_3 (`KismetMathLibrary.VSize` (- (`self.K2_GetActorLocation` _array_element_2) (`self.K2_GetActorLocation`))))
      (if (< _returnvalue_3 (`local.ClosestDist`))
        (set `local.ClosestDist` _returnvalue_3)
        (set `local.ClosestActor` _array_element_2)))
    ;[1 1 1] Return
    (if (`KismetSystemLibrary.IsValid` _closestactor)
      (if (`KismetSystemLibrary.IsValid` _returnvalue)
        (if (`/Game/Production/Blueprints/Components/BPAC_InteractableComponent.GetCanInteract` _returnvalue)
          (message `/Game/Production/Blueprints/GameMode/BPI_Interaction.OnReadyToInteract` _returnvalue)
          (return _closestactor _returnvalue)
          (else
            _))))
    (message `/Game/Production/Blueprints/HUD/BPI_HUDUtil.OnClearRenderReadyToInteractObject` (`/Game/Production/Blueprints/GameMode/BPF_GameplayUtil.GetHUD`))
    (return null null)
    (else
      ;[1 1 1] Nothing In range, return
      (return null null))))

(fn `UpdateFacingDir`
  (bind _x (.x (`CharacterMovementComponent.GetLastUpdateVelocity` (`self.CharacterMovement`))))
  (if (> (`KismetMathLibrary.Abs` _x) 0.1)
    (bind _output_get (set `self.FacingRight` (> _x 0.0)))
    (`SceneComponent.K2_SetRelativeRotation` (`self.FacingDir`) (`KismetMathLibrary.MakeRotator` 0.0 0.0 (select `bool` _output_get :`false` -180.0 :!type "Float (single-precision)")) false false)))

(fn `UserConstructionScript`)