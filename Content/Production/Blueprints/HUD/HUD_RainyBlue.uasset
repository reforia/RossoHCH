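; HUD for Rainy Blue that hosts the master UMG container and draws the ready-to-interact icon over interactable objects.
; On BeginPlay it syncs the container to the current gameplay state, then binds the GameMode's state-change delegate because initial state events may precede the HUD; cleanup events forward to the container.
; Interaction requests store a texture and projected screen position, which DrawHUD renders with a fallback texture, only during Gameplay Idle.
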(event `self.ReceiveBeginPlay`
  ;[1 1 1] Initialize an empty widget container to avoid memory leak
  (bind _returnvalue (`|CreateWidget` "/Game/Production/Blueprints/HUD/UMG_MasterContainer.UMG_MasterContainer_C" (`self.PlayerOwner`)))
  (`UserWidget.AddToViewport` _returnvalue 0)
  (set `self.MasterWidgetContainerRef` _returnvalue)
  ;[1 1 1] At this time, the GM has finished initialization, so the event has been called, we need to handle the event happened before we  even exist
  (message `/Game/Production/Blueprints/GameMode/BPI_GameplayState.InitializeOnGameplayState` (`self.MasterWidgetContainerRef`) (`/Game/Production/Blueprints/GameMode/BPF_GameplayUtil.GetRBGameplayState`))
  ;[1 1 1] Here we bind it to take care of the rest events in the future
  (add `/Game/Production/Blueprints/GameMode/GM_BP_RainyBlue.OnGameplayStateChangedDelegate` (`/Game/Production/Blueprints/GameMode/BPF_GameplayUtil.GetRBGameMode`) (delegate `HUDCustomGameplayStateChangedHandler`)))

(event `HUDCustomGameplayStateChangedHandler`
  (params (NewGameplayState :type "EGameplayState Enum" :default "EV_InGameplayIdle"))
  ;[1 1 1] Here we bind it to take care of the rest events in the future
  ;;[1 1 1] We use this instead of directly implement the interface is because we cannot guarantee that the first initialization will be finished when we are here
  (message `/Game/Production/Blueprints/GameMode/BPI_GameplayState.InitializeOnGameplayState` (`self.MasterWidgetContainerRef`) NewGameplayState))

(event `self.ReceiveTick`
  (params (DeltaSeconds :type "Float (single-precision)")))

(event `/Game/Production/Blueprints/GameMode/BPI_GameplayState.CleanUpOnGameplayState`
  (params (OldState :type "EGameplayState Enum" :default "EV_InGameplayIdle"))
  ;[1 1 1] Deconstruction is fine, since we will destroy it anyway so we directly implement interfacce
  (message `/Game/Production/Blueprints/GameMode/BPI_GameplayState.CleanUpOnGameplayState` (`self.MasterWidgetContainerRef`) OldState))

(event `RequestRenderReadyToInteract`
  (params (ActorWorldLocation :type "Vector Structure") (ReadyToInteractTexture :type "Texture Object Reference"))
  (`|ExecutionSequence`
    (:`then_0`
      ;[1 1 1] Project the item that's ready to interact from 3D coords to screen 2D coords
      (switch `EGameplayState` (`/Game/Production/Blueprints/GameMode/BPF_GameplayUtil.GetRBGameplayState`)
        (:`EV_InGameplayIdle`
          (set `self.ReadyToInteractTexture` ReadyToInteractTexture)
          (set `self.InteractableItemHUDPos` (`GameplayStatics.ProjectWorldToScreen` (`self.GetOwningPlayerController`) ActorWorldLocation))
          (set `self.RenderReadyToInteractObject` true))))))

(event `/Game/Production/Blueprints/HUD/BPI_HUDUtil.OnClearRenderReadyToInteractObject`
  (set `self.RenderReadyToInteractObject` false))

(event `self.ReceiveDrawHUD`
  (params (SizeX :type Integer) (SizeY :type Integer))
  (bind _interactableitemhudwidth (`self.InteractableItemHUDWidth`))
  (bind (_interactableitemhudpos_x _interactableitemhudpos_y) (`KismetMathLibrary.BreakVector2D` (`self.InteractableItemHUDPos`)))
  (`|ExecutionSequence`
    (:`then_0`
      (switch `EGameplayState` (`/Game/Production/Blueprints/GameMode/BPF_GameplayUtil.GetRBGameplayState`)
        (:`EV_InGameplayIdle`
          ;[1 1 1] Handle Prepare to interact HUD
          (if (`self.RenderReadyToInteractObject`)
            (`self.DrawTexture` (select `bool` (`KismetSystemLibrary.IsValid` (`self.ReadyToInteractTexture`)) :`false` "/Engine/EditorResources/Ai_Spawnpoint.Ai_Spawnpoint" :`true` (`self.ReadyToInteractTexture`)) (- _interactableitemhudpos_x (* (`self.InteractableItemHUDWidth`) 0.5)) (- _interactableitemhudpos_y (`self.InteractableItemHUDHeight`)) _interactableitemhudwidth _interactableitemhudwidth 0.0 0.0 1.0 1.0)))))))

(fn `UserConstructionScript`)