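; Blueprint function library of static accessors for core RainyBlue gameplay objects, each resolved from a world context.
; It casts to the RainyBlue game mode, reads the current gameplay state through it, and casts player 0's HUD to the RainyBlue HUD.
; The game instance and inventory service getters are thin wrappers that forward to GetGICore and GetInventoryService calls.
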(fn `GetHUD`
  (returns (HUD :type "/Game/Production/Blueprints/HUD/HUD_RainyBlue Object Reference"))
  (bind _ashud_rainy_blue (cast `/Game/Production/Blueprints/HUD/HUD_RainyBlue` (`PlayerController.GetHUD` (`GameplayStatics.GetPlayerController` (`local.__WorldContext`)))))
  (return _ashud_rainy_blue))

(fn `GetInventoryService`
  (returns (InventoryServiceRef :type "InventoryService Object Reference"))
  (return (`FuncLib_GameplayUtil.GetInventoryService` (`local.__WorldContext`))))

(fn `GetRBGameInstance`
  (returns (GIRef :type "GI_Core Object Reference"))
  (return (`FuncLib_GameplayUtil.GetGICore` (`local.__WorldContext`))))

(fn `GetRBGameMode`
  (returns (GM_RainyBlue :type "/Game/Production/Blueprints/GameMode/GM_BP_RainyBlue Object Reference"))
  (bind _asgm_bp_rainy_blue (cast `/Game/Production/Blueprints/GameMode/GM_BP_RainyBlue` (`GameplayStatics.GetGameMode` (`local.__WorldContext`)))
    (:`then`
      (return _asgm_bp_rainy_blue))
    (:`CastFailed`
      (return null))))

(fn `GetRBGameplayState`
  (returns (GameplayState :type "EGameplayState Enum"))
  (return (`GM_RainyBlue.GetCurrentGameplayState` (`self.GetRBGameMode` (`local.__WorldContext`)))))