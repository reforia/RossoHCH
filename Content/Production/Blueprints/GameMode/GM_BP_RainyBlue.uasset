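; Game mode Blueprint for RainyBlue that drives a gameplay state machine, entering InGameplayIdle on PostLogin once the player controller is ready.
; State changes initialize the player controller and then fire the state-changed delegate, while leaving a state has the HUD clean up.
; An event lets callers request state switches.
; Tick prints on-screen debug text for the current state and the inventory, quest and character services.
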(event `self.K2_PostLogin`
  (params (NewPlayer :type "PlayerController Object Reference"))
  ;[1 1 1] This needs to be delayed to PostLogin, otherwise the player controller won't be guaranteed to ready yet in memory
  (`self.SwitchGameplayState` "EV_InGameplayIdle"))

(event `self.ReceiveBeginPlay`)

(event `self.ReceiveTick`
  (params (DeltaSeconds :type "Float (single-precision)"))
  (`self.GameModeDebugInfo`))

(event `RequestSwitchGameplayState`
  (params (NewState :type "EGameplayState Enum" :default "EV_InGameplayIdle"))
  (`self.SwitchGameplayState` NewState))

(fn `GameModeDebugInfo`
  (`KismetSystemLibrary.PrintString` (`KismetStringLibrary.Concat_StrStr` "Current Gameplay State: " (`|GetEnumeratorNameAsString` (`self.GetCurrentGameplayState`))) true true (struct :`R` 1.0 :`G` 0.816077 :`A` 1.0) 0.0)
  (`KismetSystemLibrary.PrintString` (`ServiceBase.GetDebugLogInfo` (`/Game/Production/Blueprints/GameMode/BPF_GameplayUtil.GetInventoryService`)) true true (struct :`G` 0.66 :`B` 1.0 :`A` 1.0) 0.0)
  (`KismetSystemLibrary.PrintString` (`ServiceBase.GetDebugLogInfo` (`/Game/Production/Blueprints/GameMode/BPF_GameplayUtil.GetQuestService`)) true true (struct :`G` 0.66 :`B` 1.0 :`A` 1.0) 0.0)
  (`KismetSystemLibrary.PrintString` (`ServiceBase.GetDebugLogInfo` (`/Game/Production/Blueprints/GameMode/BPF_GameplayUtil.GetCharService`)) true true (struct :`G` 0.66 :`B` 1.0 :`A` 1.0) 0.0))

(fn `OnGameplayStateChanged`
  (params (newState :type "EGameplayState Enum" :default "EV_InGameplayIdle"))
  (returns (ReturnValue :type Boolean))
  (`|ExecutionSequence`
    (:`then_0`
      ;[1 1 1] PC Initialization
      (message `/Game/Production/Blueprints/GameMode/BPI_GameplayState.InitializeOnGameplayState` (`GameplayStatics.GetPlayerController` 0) newState))
    (:`then_3`
      ;[1 1 1] Call right before return to provide a updated call
      (`self.OnGameplayStateChangedDelegate` newState)
      (return false))))

(fn `OnGameplayStateDeconstructed`
  (params (oldState :type "EGameplayState Enum" :default "EV_InGameplayIdle"))
  (returns (ReturnValue :type Boolean))
  (`|ExecutionSequence`
    (:`then_0`
      ;[1 1 1] HUD Clean Up
      (message `/Game/Production/Blueprints/GameMode/BPI_GameplayState.CleanUpOnGameplayState` (`/Game/Production/Blueprints/GameMode/BPF_GameplayUtil.GetHUD`) oldState))
    (:`then_1`
      (return false))))

(fn `UserConstructionScript`)