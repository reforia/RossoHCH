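; BPAC_InventoryComponent is an actor component that connects its owner to a central inventory service.
; On BeginPlay it registers itself with the service.
; RequestPickupObject forwards an item ID and count to the service's AddObjectIntoInventory, passing itself as the caller.
; It prints on-screen warnings when the add fails or the service is invalid.
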(event `self.ReceiveBeginPlay`
  (`/Game/Production/Blueprints/GameInstance/Services/Service_Inventory.RegisterInventoryComponent` (`/Game/Production/Blueprints/GameMode/BPF_GameplayUtil.GetInventoryService`) self))

(event `RequestPickupObject`
  (params (ItemID :type Name) (Count :type Integer :default 1))
  (bind _inventoryserviceref (`/Game/Production/Blueprints/GameMode/BPF_GameplayUtil.GetInventoryService`))
  (`/Engine/EditorBlueprintResources/StandardMacros.IsValid` _inventoryserviceref
    (:`Is Valid`
      (bind _success (`/Game/Production/Blueprints/GameInstance/Services/Service_Inventory.AddObjectIntoInventory` _inventoryserviceref self ItemID Count))
      (if (not _success)
        (`KismetSystemLibrary.PrintString` "[WARNING] ITEM MODIFICATION OPERATION PERFORMED BUT FAILED" true true (struct :`R` 1.0 :`G` 0.866688 :`A` 1.0) 30.0)))
    (:`Is Not Valid`
      (`KismetSystemLibrary.PrintString` "[CRITICAL ERROR] INVENTORY SERVICE FAILED TO INITIALIZE, CHECKING GI INITIALIZATION" true true (struct :`R` 1.0 :`G` 0.028244 :`A` 1.0) 30.0))))