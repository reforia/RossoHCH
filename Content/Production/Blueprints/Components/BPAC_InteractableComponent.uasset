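; Actor component that makes its owning actor interactable.
; When ready to interact, it prints a debug string and asks the HUD to render a prompt texture at the owner's world location.
; On interaction, it clears its CanInteract flag if set to single use, then forwards the instigator to the owner through an OnInteract message.
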(event `/Game/Production/Blueprints/GameMode/BPI_Interaction.OnReadyToInteract`
  (`self.DebugReadyToBeInteracted`)
  (`/Game/Production/Blueprints/HUD/HUD_RainyBlue.RequestRenderReadyToInteract` (`/Game/Production/Blueprints/GameMode/BPF_GameplayUtil.GetHUD`) (`Actor.K2_GetActorLocation` (`self.GetOwner`)) (`self.ReadyToInteractImage`)))

(event `/Game/Production/Blueprints/GameMode/BPI_Interaction.OnInteract`
  (params (Instigator :type "Actor Object Reference"))
  (`|ExecutionSequence`
    (:`then_0`
      (if (`self.OnlyOnce`)
        (set `self.CanInteract` false)))
    (:`then_1`
      (message `/Game/Production/Blueprints/GameMode/BPI_Interaction.OnInteract` (`self.GetOwner`) Instigator))))

(fn `DebugReadyToBeInteracted`
  (`KismetSystemLibrary.PrintString` (`KismetStringLibrary.Concat_StrStr` (`KismetSystemLibrary.GetDisplayName` (`self.GetOwner`)) " ReadyToBeInteracted") true true (struct :`G` 0.66 :`B` 1.0 :`A` 1.0) 0.0))

(fn `GetCanInteract`
  (returns (CanInteract :type Boolean))
  (return (`self.CanInteract`)))