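; PC_RainyBlue is the player controller for Rainy Blue, routing player input according to the current gameplay state.
; It stores the possessed pawn and forwards move, jump and interact input to it as messages while in Gameplay Idle.
; During dialogue, Interact instead tells the HUD to finish the current dialogue line.
; Gameplay state initialization is passed on to the controlled pawn, chaining setup into the character.
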(event `self.ReceivePossess`
  (params (PossessedPawn :type "Pawn Object Reference"))
  (set `self.ControlledPawnRef` PossessedPawn))

(event `InputAxis|MoveRight`
  (params (AxisValue :type "Float (single-precision)"))
  ;[1 1 1] Control Scheme
  (switch `EGameplayState` (`/Game/Production/Blueprints/GameMode/BPF_GameplayUtil.GetRBGameplayState`)
    (:`EV_InGameplayIdle`
      (message `/Game/Production/Blueprints/GameMode/BPI_Movement.OnMoveRight` (`self.ControlledPawnRef`) AxisValue))))

(event `InputAction|Jump`
  (params (Key :type "Key Structure"))
  (:`Pressed`
    (switch `EGameplayState` (`/Game/Production/Blueprints/GameMode/BPF_GameplayUtil.GetRBGameplayState`)
      (:`EV_InGameplayIdle`
        (message `/Game/Production/Blueprints/GameMode/BPI_Movement.OnJump` (`self.ControlledPawnRef`))))))

(event `InputAction|Interact`
  (params (Key :type "Key Structure"))
  (:`Pressed`
    (switch `EGameplayState` (`/Game/Production/Blueprints/GameMode/BPF_GameplayUtil.GetRBGameplayState`)
      (:`EV_InGameplayIdle`
        (message `/Game/Production/Blueprints/GameMode/BPI_Interaction.OnInteract` (`self.ControlledPawnRef`) self))
      (:`EV_InDialogue`
        (message `/Game/Production/Blueprints/GameMode/BPI_Interaction.OnFinishCurrentDialogueLine` (`/Game/Production/Blueprints/GameMode/BPF_GameplayUtil.GetHUD`))))))

(event `/Game/Production/Blueprints/GameMode/BPI_GameplayState.InitializeOnGameplayState`
  (params (NewState :type "EGameplayState Enum" :default "EV_InGameplayIdle"))
  ;[1 1 1] Propagate Logic Chain to Char Initialization
  (message `/Game/Production/Blueprints/GameMode/BPI_GameplayState.InitializeOnGameplayState` (`self.K2_GetPawn`) NewState))

(fn `UserConstructionScript`)